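; Actor that sends a text prompt to the OpenAI Responses API and shows the reply in-game.
; SendPostRequest waits briefly, copies the Header map into a header object, prints it, and posts PostBody as JSON with the Bleach argument appended to its input.
; On success it parses the "output" field into MessageBody and passes the text to a SpawnUIElement actor's EditText.
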(event Custom|SendPostRequest
  (params (Bleach%20%25 :type String))
  (bind _postbody (Variables|Default|GetPostBody))
  (bind (_model _input) (Utilities|Struct|BreakPostBody _postbody))
  (Utilities|FlowControl|Delay 0.2)
  (CallFunction|CreateHeaders)
  (bind _outjsonstring (|StructtoJsonString (Utilities|Struct|MakePostBody _model (Utilities|String|Append _input Bleach%20%25))))
  (bind _result_body (|HttpRequest "https://api.openai.com/v1/responses" "Post" (Variables|Default|Getheaderobj) _outjsonstring)
    (:then
      (Development|PrintString "Request Procesing"))
    (:On%20Success
      (Development|PrintString "RequestSuccessful")
      (bind _outjsonobject (Class|JsonBlueprintFunctionLibrary|FromString _result_body))
      (bind _outvalue (|GetJsonField _outjsonobject "output"))
      (bind _output_get (Variables|Default|SetmessageBody (Utilities|Struct|MakeMessageBody _outvalue)))
      (bind _output_get_2 (Variables|Default|SetReply (Utilities|Struct|Breaktext (Utilities|Struct|BreakContent (Utilities|Struct|BreakMessageBody _output_get)))))
      (bind _returnvalue (Actor|GetActorOfClass "/Game/SpawnUIElement.SpawnUIElement_C"))
      (Default|EditText _returnvalue (Utilities|Text|ToText(String) _output_get_2)))
    (:On%20Error
      (Development|PrintString "Failed"))))

(event EventBeginPlay)

(event Collision|EventActorBeginOverlap
  (params (OtherActor :type Actor%20Object%20Reference)))

(event EventTick
  (params (DeltaSeconds :type Float%20%28single-precision%29)))

(fn ConstructionScript)

(fn CreateHeaders
  (bind _keys (Utilities|Map|Keys (Variables|Default|GetHeader)))
  (for (_array_element _array_index) _keys
    (bind _values (Utilities|Map|Values (Variables|Default|GetHeader)))
    (Class|HttpBlueprintFunctionLibrary|AddHeader (Variables|Default|Getheaderobj) _array_element (Utilities|Array|Get(acopy) _values _array_index)))
  (CallFunction|PrintHeaders))

(fn PrintHeaders
  (bind _outjsonstring (|StructtoJsonString (Variables|Default|Getheaderobj)))
  (Development|PrintString _outjsonstring))