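; BP_OpenAI is an actor that posts a request to the OpenAI responses API on BeginPlay and prints the outcome on screen.
; It copies the Headers map into a headers object, prints each header, and serializes the PostBody struct to JSON for the body.
; An asynchronous HTTP request node reports processing, success or failure, printing the raw response body on success without parsing it.
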(event Custom|CallOpenAIAPI
  (CallFunction|CreateHeaders)
  (bind _outjsonstring (|StructtoJsonString (Variables|Default|GetPostBody)))
  (bind _result_body (|HttpRequest "https://api.openai.com/v1/responses" "Post" (Variables|Default|GetHeadersObject) _outjsonstring)
    (:then
      (Development|PrintString "Request Processing"))
    (:On%20Success
      (Development|PrintString "Request Successful")
      (Development|PrintString _result_body true true "(R=0.000000,G=0.660000,B=1.000000,A=1.000000)" 1e+01))
    (:On%20Error
      (Development|PrintString "Request Failed"))))

(event EventBeginPlay
  (CallFunction|CallOpenAIAPI))

(event Collision|EventActorBeginOverlap
  (params (OtherActor :type Actor%20Object%20Reference)))

(event EventTick
  (params (DeltaSeconds :type Float%20%28single-precision%29)))

(fn ConstructionScript)

(fn CreateHeaders
  (bind _keys (Utilities|Map|Keys (Variables|Default|GetHeaders)))
  (for (_array_element _array_index) _keys
    (bind _values (Utilities|Map|Values (Variables|Default|GetHeaders)))
    (Class|HttpBlueprintFunctionLibrary|AddHeader (Variables|Default|GetHeadersObject) _array_element (Utilities|Array|Get(acopy) _values _array_index)))
  (CallFunction|PrintHeaders))

(fn PrintHeaders
  (for _array_element (Class|HttpBlueprintFunctionLibrary|GetAllHeaders (Variables|Default|GetHeadersObject))
    (Development|PrintString _array_element)))